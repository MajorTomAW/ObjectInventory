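; BP_Player is the player character Blueprint, with debug-style hotkeys for testing the inventory system.
; On BeginPlay it shows the mouse cursor and sets Game and UI input mode with the mouse locked.
; The F, G, H and B keys each construct an item object (pizza, cheese, rock or bag) and pass it to the inventory component's PreAddItem, targeting that component's own inventory.
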(event `self.ReceiveBeginPlay`
  (bind _asplayer_controller (cast `PlayerController` (`self.GetController`)))
  (`WidgetBlueprintLibrary.SetInputMode_GameAndUIEx` _asplayer_controller null "LockAlways" false)
  (set `PlayerController.bShowMouseCursor` true _asplayer_controller))

(event `Key|F`
  (params (Key :type "Key Structure"))
  (bind _ac_inventorycomponent (`self.AC_InventoryComponent`))
  (:`Pressed`
    ;[1 1 1] Creates the item
    (bind _returnvalue (`|GenericCreateObject` "/Game/InventorySystem/ItemObjects/IO_LargeSausagePizza.IO_LargeSausagePizza_C"))
    (`InventoryComponent.PreAddItem` _ac_inventorycomponent _returnvalue (`InventoryComponent.GetInventory` _ac_inventorycomponent))))

(event `Key|G`
  (params (Key :type "Key Structure"))
  (bind _ac_inventorycomponent (`self.AC_InventoryComponent`))
  (:`Pressed`
    (bind _returnvalue (`|GenericCreateObject` "/Game/InventorySystem/ItemObjects/IO_Cheese.IO_Cheese_C"))
    (`InventoryComponent.PreAddItem` _ac_inventorycomponent _returnvalue (`InventoryComponent.GetInventory` _ac_inventorycomponent))))

(event `Key|H`
  (params (Key :type "Key Structure"))
  (bind _ac_inventorycomponent (`self.AC_InventoryComponent`))
  (:`Pressed`
    (bind _returnvalue (`|GenericCreateObject` "/Game/InventorySystem/ItemObjects/IO_Rock.IO_Rock_C"))
    (`InventoryComponent.PreAddItem` _ac_inventorycomponent _returnvalue (`InventoryComponent.GetInventory` _ac_inventorycomponent))))

(event `Key|B`
  (params (Key :type "Key Structure"))
  (bind _ac_inventorycomponent (`self.AC_InventoryComponent`))
  (:`Pressed`
    (bind _returnvalue (`|GenericCreateObject` "/Game/InventorySystem/ItemObjects/IO_Bag.IO_Bag_C"))
    (`InventoryComponent.PreAddItem` _ac_inventorycomponent _returnvalue (`InventoryComponent.GetInventory` _ac_inventorycomponent))))

(fn `UserConstructionScript`)